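; Player controller that lets the player drag units with the cursor across a horizontal plane.
; Pressing DragUnit stores whatever actor a Visibility trace under the cursor hits, with no type filter, and opens a Tick gate; release clears it.
; Each gated tick intersects the camera-to-cursor ray with a horizontal plane at the actor's height and moves the actor there without sweeping, keeping its Z constant.
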(event `self.ReceiveTick`
  (params (DeltaSeconds :type "Float (single-precision)"))
  (bind (_worldlocation _worlddirection) (`self.DeprojectMousePositionToWorld` (`GameplayStatics.GetPlayerController` 0)))
  (`/Engine/EditorBlueprintResources/StandardMacros.Gate` true :!label _label
    (:`Exit`
      (`/Engine/EditorBlueprintResources/StandardMacros.IsValid` (stale `InputAction|DragUnit` _output_get)
        (:`Is Valid`
          (`self.K2_SetActorLocation` (`self.Hit Actor`) (`.Intersection` (`KismetMathLibrary.LinePlaneIntersection_OriginNormal` (`PlayerCameraManager.GetCameraLocation` (`GameplayStatics.GetPlayerCameraManager` 0)) (+ _worldlocation (* _worlddirection (10000.0 10000.0 10000.0))) (`self.K2_GetActorLocation` (`self.Hit Actor`)) (0.0 0.0 1.0))) false false))
        (:`Is Not Valid`
          (goto _label :!via `Close`))))))

(event `InputAction|DragUnit`
  (params (Key :type "Key Structure"))
  (bind (_bblockinghit _binitialoverlap _time _distance _location _impactpoint _normal _impactnormal _physmat _hitactor) (`GameplayStatics.BreakHitResult` (`self.GetHitResultUnderCursorByChannel` (`GameplayStatics.GetPlayerController` 0) "TraceTypeQuery1" true)))
  (:`Pressed`
    (if _bblockinghit
      (`/Engine/EditorBlueprintResources/StandardMacros.IsValid` _hitactor
        (:`Is Valid`
          (bind _output_get (set `self.Hit Actor` _hitactor))
          (goto _label :!via `Open`)))))
  (:`Released`
    (set `self.Hit Actor` null)
    (goto _label :!via `Close`)))

(fn `UserConstructionScript`)